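; HOUSE is a house actor that appears in build stages as the player character progresses.
; All three meshes start hidden, and Tick polls ThirdPersonCharacter flags to reveal the base structure and roof.
; When BoughtHouse is set, the finished mesh replaces both stages and a CongratzScreen widget is added to the viewport.
; That branch has no one-shot guard, so a new widget is created every frame while the flag holds.
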(event EventBeginPlay
  (Rendering|SetVisibility (Variables|Default|GetStaticMesh) false false))

(event Collision|EventActorBeginOverlap
  (params (OtherActor :type Actor%20Object%20Reference)))

(event EventTick
  (params (DeltaSeconds :type Float%20%28single-precision%29))
  (bind _asthird_person_character (Utilities|Casting|CastToThirdPersonCharacter (Game|GetPlayerCharacter 0)))
  (Utilities|FlowControl|Sequence
    (:then_0
      (if (Variables|/Game/ThirdPersonBP/Blueprints/ThirdPersonCharacter.ThirdPersonCharacter_C|GetBuildBase _asthird_person_character)
        (Rendering|SetVisibility (Variables|Default|GetBaseStructure) true false)))
    (:then_1
      (if (Variables|/Game/ThirdPersonBP/Blueprints/ThirdPersonCharacter.ThirdPersonCharacter_C|GetBuildRoof _asthird_person_character)
        (Rendering|SetVisibility (Variables|Default|GetRoof) true false)))
    (:then_2
      (if (Variables|/Game/ThirdPersonBP/Blueprints/ThirdPersonCharacter.ThirdPersonCharacter_C|GetBoughtHouse _asthird_person_character)
        (Rendering|SetVisibility (Variables|Default|GetStaticMesh) true false)
        (Rendering|SetVisibility (Variables|Default|GetBaseStructure) false false)
        (Rendering|SetVisibility (Variables|Default|GetRoof) false false)
        (bind _returnvalue (UserInterface|CreateWidget "/Game/UI/CongratzScreen.CongratzScreen_C"))
        (UserInterface|Viewport|AddtoViewport _returnvalue 0)))))

(fn ConstructionScript
  (Rendering|SetVisibility (Variables|Default|GetRoof) false false))